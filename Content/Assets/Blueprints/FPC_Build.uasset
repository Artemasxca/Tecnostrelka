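; FPC_Build is a player Blueprint, apparently a first-person character, that hosts the main menu, pause menu and position saving.
; BeginPlay opens WBP_Menu with UI-only input and a visible cursor, and the Pause action does the same with WBP_Pause, guarded by IsPaused.
; SaveGame writes the actor transform to a BP_Save slot and prints a confirmation; LoadGame restores that transform.
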(event Custom|SaveGame
  (bind _returnvalue (SaveGame|CreateSaveGameObject "/Game/Assets/Blueprints/BP_Save.BP_Save_C"))
  (Variables|/Game/Assets/Blueprints/BP_Save.BP_Save_C|SetPlayerPosition _returnvalue (Transformation|GetActorTransform))
  (SaveGame|SaveGametoSlot _returnvalue "save")
  (Development|PrintText "Сохранено"))

(event Custom|LoadGame
  (bind _returnvalue (SaveGame|LoadGamefromSlot "save"))
  (bind _asbp_save (Utilities|Casting|CastToBP_Save _returnvalue))
  (Transformation|SetActorTransform (Variables|/Game/Assets/Blueprints/BP_Save.BP_Save_C|GetPlayerPosition _asbp_save)))

(event EventBeginPlay
  (bind _returnvalue (Game|GetPlayerController 0))
  (Input|SetInputModeUIOnly _returnvalue 0 "DoNotLock" false)
  (Variables|/Script/Engine.PlayerController|SetbShowMouseCursor _returnvalue true)
  (bind _returnvalue_2 (UserInterface|CreateWidget "/Game/Assets/UI/WBP_Menu.WBP_Menu_C"))
  (bind _output_get (Variables|Default|SetMainMenuRef _returnvalue_2))
  (UserInterface|Viewport|AddtoViewport _output_get 0))

(event Collision|EventActorBeginOverlap
  (params (OtherActor :type Actor%20Object%20Reference)))

(event EventTick
  (params (DeltaSeconds :type Float%20%28single-precision%29)))

(event Input|ActionEvents|InputActionPause
  (params (Key :type Key%20Structure :default "None"))
  (bind _returnvalue (Game|GetPlayerController 0))
  (:Pressed
    (if (not (Variables|Default|GetIsPaused?))
      (Input|SetInputModeUIOnly _returnvalue 0 "DoNotLock" false)
      (Variables|/Script/Engine.PlayerController|SetbShowMouseCursor _returnvalue true)
      (bind _returnvalue_2 (UserInterface|CreateWidget "/Game/Assets/UI/WBP_Pause.WBP_Pause_C"))
      (UserInterface|Viewport|AddtoViewport _returnvalue_2 0)
      (Variables|Default|SetIsPaused? true))))

(fn ConstructionScript
  (|CallParentFunction))