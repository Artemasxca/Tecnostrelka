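; Building tool component that spawns a preview A_Builds actor from a selected data asset and positions it for placement via Enhanced Input.
; Each Tick, unless frozen, a camera line trace moves the preview freely or on a grid, then checks placement validity.
; Snap mode aligns a scroll-selected snap point against the closest one on the targeted build.
; A sphere trace with set differences shows and hides nearby builds' snap points.
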(event Input|EnhancedActionEvents|EnhancedInputActionIA_BuildSelect
  (params (ActionValue :type Float%20%28double-precision%29) (ElapsedSeconds :type Float%20%28double-precision%29) (TriggeredSeconds :type Float%20%28double-precision%29) (InputAction :type Input%20Action%20Object%20Reference :default "/Game/Assets/Input/IA_BuildSelect.IA_BuildSelect"))
  (:Started
    (CallFunction|SpawnNewBuild (.Value (Utilities|Map|Find (Variables|Default|GetBuildingMap) (Math|Float|Round ActionValue))))))

(event Input|EnhancedActionEvents|EnhancedInputActionIA_Grid
  (params (ActionValue :type Boolean) (ElapsedSeconds :type Float%20%28double-precision%29) (TriggeredSeconds :type Float%20%28double-precision%29) (InputAction :type Input%20Action%20Object%20Reference :default "/Game/Assets/Input/IA_Grid.IA_Grid"))
  (:Started
    (Variables|Default|SetIsUsingGrid true)
    (bind _buildinreference (Variables|Default|GetBuildinReference)
      (:then
        (Transformation|SetActorRotation _buildinreference (Math|Rotator|MakeRotator (.roll (Transformation|GetActorRotation _buildinreference)) (.pitch (Transformation|GetActorRotation _buildinreference)) (Math|Float|SnapToGrid(Float) (.yaw (Transformation|GetActorRotation _buildinreference)) 9e+01))))
      (:else)))
  (:Canceled
    (Variables|Default|SetIsUsingGrid false :!label _label))
  (:Completed
    (goto _label)))

(event Input|EnhancedActionEvents|EnhancedInputActionIA_Rotate
  (params (ActionValue :type Float%20%28double-precision%29) (ElapsedSeconds :type Float%20%28double-precision%29) (TriggeredSeconds :type Float%20%28double-precision%29) (InputAction :type Input%20Action%20Object%20Reference :default "/Game/Assets/Input/IA_Rotate.IA_Rotate"))
  (bind _isusinggrid (Variables|Default|GetIsUsingGrid))
  (bind _returnvalue (Math|Float|SelectFloat 9e+01 45.0 _isusinggrid))
  (:Started
    (bind _buildinreference (Variables|Default|GetBuildinReference)
      (:then
        (if (Variables|Default|GetIsSnapping)
          (|ModifyCounter (> ActionValue 0.0))
          (else
            (Class|Actor|AddActorWorldRotation _buildinreference (Math|Rotator|MakeRotator 0.0 0.0 (Math|Float|MapRangeClamped ActionValue -1.0 0.0 (* _returnvalue -1.0) _returnvalue))))))
      (:else))))

(event Input|EnhancedActionEvents|EnhancedInputActionIA_Confirm
  (params (ActionValue :type Boolean) (ElapsedSeconds :type Float%20%28double-precision%29) (TriggeredSeconds :type Float%20%28double-precision%29) (InputAction :type Input%20Action%20Object%20Reference :default "/Game/Assets/Input/IA_Confirm.IA_Confirm"))
  (:Started
    (bind _buildinreference (Variables|Default|GetBuildinReference)
      (:then
        (if (Variables|/Game/Assets/Blueprints/A_Builds.A_Builds_C|GetIsValidPlacement _buildinreference)
          (Default|PlaceBuilding (Variables|Default|GetBuildinReference))
          (Variables|Default|SetBuildinReference 0)))
      (:else))))

(event Input|EnhancedActionEvents|EnhancedInputActionIA_Snap
  (params (ActionValue :type Boolean) (ElapsedSeconds :type Float%20%28double-precision%29) (TriggeredSeconds :type Float%20%28double-precision%29) (InputAction :type Input%20Action%20Object%20Reference :default "/Game/Assets/Input/IA_Snap.IA_Snap"))
  (:Triggered
    (CallFunction|DisplaySnapPoint))
  (:Started
    (Variables|Default|SetIsSnapping true)
    (bind _buildinreference (Variables|Default|GetBuildinReference)
      (:then
        (Default|ShowSnap _buildinreference))
      (:else)))
  (:Canceled
    (Variables|Default|SetIsSnapping false :!label _label)
    (bind _result (Utilities|Set|ToArray (Variables|Default|GetBuidsInRange)))
    (for _array_element _result
      (Default|HideSnap _array_element))
    (Utilities|Set|Clear (Variables|Default|GetBuidsInRange)))
  (:Completed
    (goto _label)))

(event Input|EnhancedActionEvents|EnhancedInputActionIA_Freeze
  (params (ActionValue :type Boolean) (ElapsedSeconds :type Float%20%28double-precision%29) (TriggeredSeconds :type Float%20%28double-precision%29) (InputAction :type Input%20Action%20Object%20Reference :default "/Game/Assets/Input/IA_Freeze.IA_Freeze"))
  (:Started
    (if (Variables|Default|GetIsFrozen)
      (Variables|Default|SetIsFrozen false)
      (else
        (Variables|Default|SetIsFrozen true)))))

(event EventBeginPlay
  (Input|AddMappingContext (PlayerController|LocalPlayerSubsystems|GetEnhancedInputLocalPlayerSubsystem (Game|GetPlayerController 0)) "/Game/Assets/Input/IMC_Building.IMC_Building" 0 "(bIgnoreAllPressedKeysUntilRelease=True,bForceImmediately=False,bNotifyUserSettings=False)"))

(event EventTick
  (params (DeltaSeconds :type Float%20%28single-precision%29))
  (if (not (Variables|Default|GetIsFrozen))
    (CallFunction|UpdateBuildLocation)))

(fn SpawnNewBuild
  (params (InputPin :type DA%20Blueprint%20Soft%20Object%20Reference))
  (bind _returnvalue (Components|GetOwner))
  (bind _buildinreference (Variables|Default|GetBuildinReference)
    (:then
      (Actor|DestroyActor _buildinreference))
    (:else
      _))
  (bind _outhit (Utilities|LineTracebyChanell))
  (bind _returnvalue_2 (Game|SpawnActorfromClass "/Game/Assets/Blueprints/A_Builds.A_Builds_C" (Math|Transform|MakeTransform (.ImpactPoint (Collision|BreakHitResult _outhit)) (Transformation|GetActorRotation _returnvalue) "1.000000,1.000000,1.000000") "Undefined" "MultiplyWithRoot" 0 InputPin (.AsPawn (Utilities|Casting|CastToPawn _returnvalue))))
  (Variables|Default|SetBuildinReference _returnvalue_2)
  (Variables|Default|SetIsFrozen false))

(fn UpdateBuildLocation
  (bind _buildinreference (Variables|Default|GetBuildinReference))
  (Variables|Default|GetBuildinReference
    (:then
      (Utilities|FlowControl|Sequence
        (:then_0
          (if (not (Variables|Default|GetIsSnapping))
            (bind _outhit (Utilities|LineTracebyChanell))
            (Transformation|SetActorLocation (Variables|Default|GetBuildinReference) (Math|Vector|SelectVector (Class|KismetMathLibrary|VectorSnappedtoGrid (.ImpactPoint (Collision|BreakHitResult _outhit)) 5e+02) (.ImpactPoint (Collision|BreakHitResult _outhit)) (Variables|Default|GetIsUsingGrid)) false false)
            (else
              (bind _outhit_2 (Utilities|LineTracebyChanell))
              (LocalVariables|SetL-ImpactPoint (- (.ImpactPoint (Collision|BreakHitResult _outhit_2)) (.Normal (Collision|BreakHitResult _outhit_2))))
              (bind _asa_builds (Utilities|Casting|CastToA_Builds (.HitActor (Collision|BreakHitResult _outhit_2)))
                (:then
                  (bind _output_get (LocalVariables|SetL-HitActor _asa_builds))
                  (bind _returnvalue (Default|GetClosestTransform _output_get (LocalVariables|GetL-ImpactPoint) (Variables|/Game/Assets/Blueprints/A_Builds.A_Builds_C|GetDataAssetUsed (Variables|Default|GetBuildinReference))))
                  (LocalVariables|SetL-SnapPoint _returnvalue)
                  (if (or (Utilities|Operators|NotEqual(!=) (.location (LocalVariables|GetL-SnapPoint)) (Math|Transform|TransformLocation (Transformation|GetActorTransform (Variables|Default|GetBuildinReference)) (.location (.snappoint (Utilities|Array|Get(acopy) (Variables|/Game/Assets/Blueprints/A_Builds.A_Builds_C|GetSnapPointFilter _buildinreference) (Variables|/Game/Assets/Blueprints/A_Builds.A_Builds_C|GetSelectedIndex _buildinreference))))) 0.0) (!= (Variables|/Game/Assets/Blueprints/A_Builds.A_Builds_C|GetSelectedIndex (Variables|Default|GetBuildinReference)) (Variables|Default|GetScrolledInteger)))
                    (Transformation|SetActorRotation (Variables|Default|GetBuildinReference) (Math|Rotator|MakeRotfromX (* (Math|Vector|GetForwardVector (Math|Transform|TransformRotation (LocalVariables|GetL-SnapPoint) (.rotation (.snappoint (Utilities|Array|Get(acopy) (Variables|/Game/Assets/Blueprints/A_Builds.A_Builds_C|GetSnapPointFilter (Variables|Default|GetBuildinReference)) (Variables|Default|GetScrolledInteger)))))) -1.0)))
                    (Transformation|AddActorWorldOffset (Variables|Default|GetBuildinReference) (- (.location (LocalVariables|GetL-SnapPoint)) (Math|Transform|TransformLocation (Transformation|GetActorTransform (Variables|Default|GetBuildinReference)) (.location (.snappoint (Utilities|Array|Get(acopy) (Variables|/Game/Assets/Blueprints/A_Builds.A_Builds_C|GetSnapPointFilter (Variables|Default|GetBuildinReference)) (Variables|Default|GetScrolledInteger)))))))
                    (Variables|/Game/Assets/Blueprints/A_Builds.A_Builds_C|SetSelectedIndex (Variables|Default|GetBuildinReference) (Variables|Default|GetScrolledInteger))))
                (:CastFailed
                  (Transformation|SetActorLocation (Variables|Default|GetBuildinReference) (LocalVariables|GetL-ImpactPoint) false false)
                  (LocalVariables|SetL-HitActor 0))))))
        (:then_1
          (Default|CanPlaceBuild (Variables|Default|GetBuildinReference)))))
    (:else)))

(fn DisplaySnapPoint
  (bind _returnvalue (Game|GetPlayerCameraManager 0))
  (bind _returnvalue_2 (Transformation|GetActorLocation _returnvalue))
  (bind _outhits (Collision|MultiSphereTraceByChannel _returnvalue_2 _returnvalue_2 (Variables|Default|GetRange) "TraceTypeQuery1" false 0 "ForOneFrame"))
  (for _array_element _outhits
    (bind _asa_builds (Utilities|Casting|CastToA_Builds (.HitActor (Collision|BreakHitResult _array_element))))
    (Utilities|Set|Add (LocalVariables|GetL_HitBuilds) _asa_builds))
  (if (Utilities|Set|IsEmpty (Variables|Default|GetBuidsInRange))
    (bind _output_get (Variables|Default|SetBuidsInRange (LocalVariables|GetL_HitBuilds)))
    (bind _result (Utilities|Set|ToArray _output_get))
    (for _array_element_2 _result
      (Default|ShowSnap _array_element_2))
    (else
      (Utilities|FlowControl|Sequence
        (:then_0
          (bind _result_2 (Utilities|Set|Difference (Variables|Default|GetBuidsInRange) (LocalVariables|GetL_HitBuilds)))
          (bind _result_3 (Utilities|Set|ToArray _result_2))
          (for _array_element_3 _result_3
            (Default|HideSnap _array_element_3)))
        (:then_1
          (bind _result_4 (Utilities|Set|Difference (LocalVariables|GetL_HitBuilds) (Variables|Default|GetBuidsInRange)))
          (bind _result_5 (Utilities|Set|ToArray _result_4))
          (for _array_element_4 _result_5
            (Default|ShowSnap _array_element_4)))
        (:then_2
          (Variables|Default|SetBuidsInRange (LocalVariables|GetL_HitBuilds)))))))